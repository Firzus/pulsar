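; BP_Note is a rhythm-game lane note that moves along negative Y at its note speed while active.
; InitializeNote stores note data, speed and game mode, then places it at the lane's X and the passed target Y, kept in TargetX.
; Tick calls OnHit with Perfect, not Miss, once Y drops below TargetX.
; OnHit deactivates the note and dispatches to Perfect, Good or Miss effect functions, all empty stubs.
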(event `self.ReceiveBeginPlay`
  (bind _returnvalue_x (`KismetMathLibrary.BreakVector` (`self.K2_GetActorLocation`)))
  (bind (_notedata_hittime _notedata_lane) (break `/Game/Core/Data/Structs/S_NoteData` (`self.NoteData`)))
  (set `self.DefaultMaterial` "/Engine/MapTemplates/Materials/BasicAsset01.BasicAsset01")
  (set `self.TargetX` _returnvalue_x)
  (`KismetSystemLibrary.PrintText` (`|FormatText` "Note Lane {0} spawned at X={1}" (`KismetTextLibrary.Conv_IntToText` _notedata_lane) (`self.TargetX`))))

(event `self.ReceiveTick`
  (params (DeltaSeconds :type "Float (single-precision)"))
  (if (`self.IsActive`)
    (`self.UpdateMovement` DeltaSeconds)
    (bind _haspassed (`self.AutoMiss`))
    (if _haspassed
      (`self.OnHit` "NewEnumerator0"))))

(event `self.HitZone.OnComponentHit`
  (params (HitComponent :type "PrimitiveComponent Object Reference") (OtherActor :type "Actor Object Reference") (OtherComp :type "PrimitiveComponent Object Reference") (NormalImpulse :type "Vector Structure") (Hit :type "HitResult Structure (by ref)")))

(fn `AutoMiss`
  (returns (HasPassed :type Boolean))
  (bind (_returnvalue_x _returnvalue_y) (`KismetMathLibrary.BreakVector` (`self.K2_GetActorLocation`)))
  (return (< _returnvalue_y (`self.TargetX`))))

(fn `InitializeNote`
  (params (`Note Data` :type "/Game/Core/Data/Structs/S_NoteData Structure") (Speed :type "Float (double-precision)") (TargetYPosition :type "Float (double-precision)") (GameModeReference :type "/Game/Core/Blueprints/BP_GameMode Object Reference"))
  (bind (_gameplaysettings_notespeed _gameplaysettings_lanewidth _gameplaysettings_lanepositions) (break `/Game/Core/Data/Structs/S_GameplaySettings` (`/Game/Core/Blueprints/BP_GameMode.GameplaySettings` (`self.GameModeRef`))))
  (bind _output_get (set `self.NoteData` `Note Data`))
  (set `self.NoteSpeed` Speed)
  (set `self.TargetX` TargetYPosition)
  (set `self.GameModeRef` GameModeReference)
  (`self.K2_SetActorLocation` (`KismetMathLibrary.MakeVector` (`|GetArrayItem` _gameplaysettings_lanepositions (`.Lane_5_5F330C584A8A4810B9277D8161819D39` (break `/Game/Core/Data/Structs/S_NoteData` _output_get))) (`self.TargetX`))))

(fn `OnHit`
  (params (JudgmentType :type "/Game/Core/Data/Enums/E_JudgmentType Enum" :default "NewEnumerator0"))
  (set `self.HasBeenHit` true)
  (set `self.IsActive` false)
  (switch `/Game/Core/Data/Enums/E_JudgmentType` JudgmentType
    (:`NewEnumerator0`
      (`self.PlayPerfectEffect`))
    (:`NewEnumerator1`
      (`self.PlayGoodEffect`))
    (:`NewEnumerator3`
      (`self.PlayMissEffect`))))

(fn `PlayGoodEffect`)

(fn `PlayMissEffect`)

(fn `PlayPerfectEffect`)

(fn `UpdateMovement`
  (params (DeltaTime :type "Float (double-precision)"))
  (bind (_returnvalue_x _returnvalue_y) (`KismetMathLibrary.BreakVector` (`self.K2_GetActorLocation`)))
  (`self.K2_SetActorLocation` (`KismetMathLibrary.MakeVector` 0.0 (- _returnvalue_y (* DeltaTime (`self.NoteSpeed`))))))

(fn `UserConstructionScript`)