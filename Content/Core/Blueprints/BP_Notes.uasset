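; BP_Notes is a single note actor in a rhythm game that scrolls along Z through a judgement line.
; On BeginPlay it caches the BP_GameManager.
; Each Tick it recomputes its position from the manager's current time, placing X by column and Z by time offset and scroll speed, so movement follows the game clock.
; A time-based visibility reveal is present but disconnected.
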(event `self.ReceiveBeginPlay`
  (bind _returnvalue (`GameplayStatics.GetActorOfClass` "/Game/Core/Blueprints/BP_GameManager.BP_GameManager_C"))
  (set `self.GameManager` _returnvalue))

(event `self.ReceiveTick`
  (params (DeltaSeconds :type "Float (single-precision)"))
  (bind _notedata_time (break `/Game/Core/Blueprints/NoteData` (`self.NoteData`)))
  (bind (_notedata_time_2 _notedata_column) (break `/Game/Core/Blueprints/NoteData` (`self.NoteData`)))
  (`|ExecutionSequence`
    (:`then_0`
      (bind _newparam (`/Game/Core/Blueprints/BP_GameManager.GetCurrentTime` (`self.GameManager`)))
      (set `self.RemainingTime` (- _newparam _notedata_time))
      (`self.K2_SetActorLocation` (`KismetMathLibrary.MakeVector` (`KismetMathLibrary.Conv_IntToDouble` (* _notedata_column 100)) 0.0 (+ (`self.JudgementLineZ`) (* (* (`self.ScrollSpeed`) (`self.RemainingTime`)) -1.0)))))))

(fn `UserConstructionScript`)