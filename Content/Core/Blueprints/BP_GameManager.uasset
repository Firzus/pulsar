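; BP_GameManager runs a rhythm game's chart clock and triggers note spawning.
; On BeginPlay it finds the BP_NotesSpawner and starts the chart, recording real time as the song's start.
; Each tick it updates CurrentTime while playing, then scans CurrentChartData and spawns each note entering the TimeBeforeSpawn lead window, tracking spawned indices so each spawns once.
; GetCurrentTime exposes the chart clock.
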(event `StartChart`
  (set `self.StartTime` (`GameplayStatics.GetRealTimeSeconds`))
  (set `self.IsPlaying` true))

(event `self.ReceiveBeginPlay`
  (bind _returnvalue (`GameplayStatics.GetActorOfClass` "/Game/Core/Blueprints/BP_NotesSpawner.BP_NotesSpawner_C"))
  (set `self.NoteSpawner` _returnvalue)
  (`self.StartChart`))

(event `self.ReceiveTick`
  (params (DeltaSeconds :type "Float (single-precision)"))
  (`|ExecutionSequence`
    (:`then_0`
      (if (`self.IsPlaying`)
        (set `self.CurrentTime` (- (`GameplayStatics.GetRealTimeSeconds`) (`self.StartTime`)))))
    (:`then_1`
      (for (_array_element _array_index) (`self.CurrentChartData`)
        (if (`KismetArrayLibrary.Array_Contains` (`self.SpawnIndices`) _array_index)
          _
          (elif (<= (- (break `/Game/Core/Blueprints/NoteData` _array_element) (`self.CurrentTime`)) (`self.TimeBeforeSpawn`))
            (`/Game/Core/Blueprints/BP_NotesSpawner.SpawnNote` (`self.NoteSpawner`) (make `/Game/Core/Blueprints/NoteData` (break `/Game/Core/Blueprints/NoteData` _array_element) (`.Column_5_453A12E64A9CC5C9561449A4AF7C736F` (break `/Game/Core/Blueprints/NoteData` _array_element)) (`.Type_8_4FD929CA4BE0ED24654AA8BF306C816A` (break `/Game/Core/Blueprints/NoteData` _array_element))))
            (`KismetArrayLibrary.Array_Add` (`self.SpawnIndices`) _array_index)))))))

(fn `GetCurrentTime`
  (returns (NewParam :type "Float (double-precision)"))
  (return (`self.CurrentTime`)))

(fn `UserConstructionScript`)